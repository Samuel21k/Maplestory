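; Base 2D player character for a Maplestory-style game, handling movement, jumping and flipbook animation through Enhanced Input.
; Movement input sends a movement state to the server, and its RepNotify flips the sprite and picks flipbooks from PlayerInfo.
; Jumping bypasses that state: it sets hardcoded flipbooks locally, blocks movement input, and polls vertical velocity on a delay loop to detect landing.
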(event Custom|SetMovementState
  (params (MovementState :type E_MovementState%20Enum :default "NewEnumerator0"))
  (CallFunction|SRVSetMovementState MovementState))

(event Custom|SRV_SetMovementState
  (params (MovementState :type E_MovementState%20Enum :default "NewEnumerator0"))
  (Variables|Default|SetMovementState MovementState))

(event Input|EnhancedActionEvents|EnhancedInputActionIA_Movement
  (params (ActionValue :type Float%20%28double-precision%29) (ElapsedSeconds :type Float%20%28double-precision%29) (TriggeredSeconds :type Float%20%28double-precision%29) (InputAction :type Input%20Action%20Object%20Reference :default "/Game/Blueprints/IA_Movement.IA_Movement"))
  (:Triggered
    (if (not (Variables|Default|GetPIsJumping))
      (Pawn|Input|AddMovementInput (Transformation|GetActorForwardVector) ActionValue false)
      (if (> ActionValue 0.0)
        (CallFunction|SetMovementState "NewEnumerator1")
        (else
          (CallFunction|SetMovementState "NewEnumerator2")))))
  (:Completed
    (if (not (Variables|Default|GetPIsJumping))
      (CallFunction|SetMovementState "NewEnumerator0"))))

(event Input|EnhancedActionEvents|EnhancedInputActionIA_Jump
  (params (ActionValue :type Float%20%28double-precision%29) (ElapsedSeconds :type Float%20%28double-precision%29) (TriggeredSeconds :type Float%20%28double-precision%29) (InputAction :type Input%20Action%20Object%20Reference :default "/Game/Blueprints/IA_Jump.IA_Jump"))
  (bind _sprite (Variables|Default|GetSprite))
  (:Triggered
    (if (not (Variables|Default|GetPIsJumping))
      (Variables|Default|SetPIsJumping true)
      (Character|Jump)
      (Components|Timeline|SetLooping _sprite false)
      (Sprite|SetFlipbook _sprite "/Game/Assets/Characters/Serena/S_FP_Jump.S_FP_Jump")
      (Utilities|FlowControl|Delay 0.1)
      (if (== (.Z (Math|Vector|BreakVector (Transformation|GetVelocity))) 0.0) :!label _label
        (Components|Timeline|SetLooping _sprite true)
        (Audio|Components|Audio|Play _sprite)
        (Sprite|SetFlipbook _sprite "/Game/Assets/Characters/Serena/S_FP_Idle.S_FP_Idle")
        (Variables|Default|SetPIsJumping false)
        (else
          (Utilities|FlowControl|Delay 0.1)
          (goto _label))))))

(event EventBeginPlay
  (bind _aspc_maplestory (Utilities|Casting|CastToPC_Maplestory (Pawn|GetController)))
  (Input|AddMappingContext (PlayerController|LocalPlayerSubsystems|GetEnhancedInputLocalPlayerSubsystem _aspc_maplestory) "/Game/Blueprints/IMC_Default.IMC_Default" 0 "(bIgnoreAllPressedKeysUntilRelease=True,bForceImmediately=False)"))

(fn ConstructionScript
  (|CallParentFunction))

(fn FIsNotJumping
  (return (not (AI|Components|NavMovement|IsFalling (Variables|Character|GetCharacterMovement)))))

(fn OnRepMovementState
  (bind _sprite (Variables|Default|GetSprite))
  (bind _playerinfo (Variables|Default|GetPlayerInfo))
  (bind (_idleanimation _runanimation _jumpanimation _fallanimation) (Utilities|Struct|BreakST_PlayerInfo _playerinfo))
  (switch Utilities|FlowControl|Switch|SwitchonE_MovementState (Variables|Default|GetMovementState)
    (:NewEnumerator0
      (Sprite|SetFlipbook _sprite _idleanimation))
    (:NewEnumerator1
      (Transformation|SetRelativeRotation _sprite "0, 0, 0" false false)
      (Sprite|SetFlipbook (Variables|Default|GetSprite) _runanimation))
    (:NewEnumerator2
      (Transformation|SetRelativeRotation _sprite "0.000000,-180.000000,0.000000" false false)
      (Sprite|SetFlipbook (Variables|Default|GetSprite) _runanimation))
    (:NewEnumerator4
      (Sprite|SetFlipbook _sprite _jumpanimation))
    (:NewEnumerator3
      (Sprite|SetFlipbook _sprite _fallanimation))))